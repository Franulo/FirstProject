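; BP_WaveSpawner spawns escalating waves of BP_Enemy actors, starting the first on BeginPlay.
; SpawnWave increments CurrentWave, reads that wave's enemy count from the Waves map values by index, and spawns each enemy at a random SpawnPositions entry.
; CheckforEnemies, not called within this Blueprint, plays the Completed sound and starts the next wave when no BP_Enemy actors remain.
; Nothing guards against running past the last wave.
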(event Custom|Spawn%20Wave
  ;[0.25 0.25 0.25] Spawn Wave
  (Math|Integer|IncrementInt (Variables|Default|GetCurrent%20Wave)
    (:%20%20
      (bind _values (Utilities|Map|Values (Variables|Default|GetWaves)))
      (for _index (range 1 (Utilities|Array|Get(acopy) _values (- (Variables|Default|GetCurrent%20Wave) 1)))
        (Game|SpawnActorfromClass "/Game/Blueprints/BP_Enemy.BP_Enemy_C" (.OutItem (Utilities|Array|Random (Variables|Default|GetSpawn%20Positions))) "AdjustIfPossibleButAlwaysSpawn" "MultiplyWithRoot" 0 0)))))

(event Custom|Check%20for%20Enemies
  ;[0.25 0.25 0.25] Spawn New Wave
  (bind _outactors (Actor|GetAllActorsOfClass "/Game/Blueprints/BP_Enemy.BP_Enemy_C"))
  (if (== (Utilities|Array|Length _outactors) 0)
    (Audio|PlaySound2D "/Game/Audio/Completed.Completed" 1.0 1.0 0.0 0 0)
    (CallFunction|SpawnWave)))

(event EventBeginPlay
  (CallFunction|SpawnWave))

(fn ConstructionScript)