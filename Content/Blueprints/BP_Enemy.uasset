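; Enemy character that chases the player, makes melee attacks and notifies BP_WaveSpawner after it dies.
; ChasePlayer loops AI MoveTo into a push montage, whose notify triggers a forward sphere trace that applies damage, with CanAttack gating each attack.
; Damage plays a grunt and either knocks it back or runs death: montage, collision and movement off, delayed destroy, then CheckForEnemies.
; A random-roam Wonder loop exists but nothing here calls it.
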(event Custom|Wonder
  ;[0.25 0.25 0.25] Wonder
  (AI|AIMoveTo self (.RandomLocation (AI|Navigation|GetRandomReachablePointinRadius (Transformation|GetActorLocation) 5e+02 0 0)) 0 5.0 false
    (:OnSuccess
      (Utilities|FlowControl|Delay 1.0)
      (CallFunction|Wonder))))

(event Custom|Chase%20Player
  (bind _attacktracepos (Variables|Default|GetAttackTracePos))
  (bind _returnvalue (Transformation|GetWorldLocation _attacktracepos))
  ;[0.25 0.25 0.25] Case and Attack Player
  (AI|AIMoveTo self "0, 0, 0" (Game|GetPlayerCharacter 0) 5.0 false
    (:OnSuccess
      (if (Variables|Default|Getcan%20Attack)
        (Animation|Montage|PlayMontage (Variables|Character|GetMesh) "/Game/Characters/Mannequin_UE4/OurAnimation/Push_Montage.Push_Montage"
          (:then
            (Variables|Default|Setcan%20Attack false))
          (:OnCompleted
            (Variables|Default|Setcan%20Attack true)
            (CallFunction|ChasePlayer))
          (:OnNotifyBegin
            (bind (_outhit _returnvalue_2) (Collision|SphereTraceForObjects _returnvalue (+ (* (Math|Vector|GetForwardVector _attacktracepos) 1e+02) _returnvalue) 25.0 (Utilities|Array|MakeArray "ObjectTypeQuery3") false 0 "None"))
            (if _returnvalue_2
              (Game|Damage|ApplyDamage (.HitActor (Collision|BreakHitResult _outhit)) 1e+01 0 0))))))))

(event Game|Damage|EventAnyDamage
  (params (Damage :type Float%20%28single-precision%29) (DamageType :type Damage%20Type%20Object%20Reference) (InstigatedBy :type Controller%20Object%20Reference) (DamageCauser :type Actor%20Object%20Reference))
  ;[0.25 0.25 0.25] DamageTaken
  (Variables|Default|SetHealth (- (Variables|Default|GetHealth) Damage))
  (Audio|PlaySoundatLocation "/Game/Audio/MS_DamageGrunt.MS_DamageGrunt" (Transformation|GetActorLocation) "0, 0, 0" 1.0 1.0 0.0 0 0 0 0)
  (if (<= (Variables|Default|GetHealth) 0.0)
    (Animation|Montage|PlayMontage (Variables|Character|GetMesh) "/Game/Characters/Mannequins/Animations/Manny/AM_Dead.AM_Dead"
      (:then
        (Variables|Default|Setcan%20Attack false)
        (Collision|SetActorEnableCollision false)
        (Pawn|Components|CharacterMovement|DisableMovement (Variables|Character|GetCharacterMovement))
        (Utilities|FlowControl|Delay 3.0)
        (Actor|DestroyActor)
        (bind _outactors (Actor|GetAllActorsOfClass "/Game/Blueprints/BP_WaveSpawner.BP_WaveSpawner_C"))
        (Default|CheckforEnemies _outactors)))
    (else
      (Character|LaunchCharacter (+ (* (Transformation|GetActorForwardVector) -2e+02) (* (Transformation|GetActorUpVector) 1e+02)) false false))))

(event EventBeginPlay
  (CallFunction|ChasePlayer))

(fn ConstructionScript)